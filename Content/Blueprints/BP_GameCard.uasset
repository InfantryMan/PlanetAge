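; BP_GameCard is an actor that displays a planet, with a name label, a shape mesh and a table mesh.
; The construction script applies the planet name and uses PlanetStruct to set the shape's material and uniform scale.
; A dynamic material instance tints the table with the planet's color.
; The ChangeCardScale event calls ChangeSize to shrink the shape by a fixed factor, compounding with each call.
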(event EventBeginPlay)

(event Collision|EventActorBeginOverlap
  (params (OtherActor :type Actor%20Object%20Reference)))

(event EventTick
  (params (DeltaSeconds :type Float%20%28single-precision%29)))

(event Custom|ChangeCardScale
  (CallFunction|ChangeSize 0.9))

(fn ConstructionScript
  (bind _gamecardshape (Variables|Default|GetGameCardShape))
  (bind _planetstruct (Variables|Default|GetPlanetStruct))
  (bind (_material _color _planetscale) (Utilities|Struct|BreakPlanetStruct _planetstruct))
  (Rendering|Components|TextRender|SetText (Variables|Default|GetNameComponent) (Utilities|Text|ToText(String) (Variables|Default|GetPlanetName)))
  (Rendering|Material|SetMaterial _gamecardshape 0 _material)
  (Transformation|SetWorldScale3D _gamecardshape (Math|Vector|MakeVector _planetscale _planetscale _planetscale))
  (bind _returnvalue (Rendering|Material|CreateDynamicMaterialInstance "/Game/Materials/NoColor.NoColor" "None" :!class /Script/Engine.KismetMaterialLibrary))
  (bind _output_get (Variables|Default|SetTableComponentDynamicMI _returnvalue))
  (Rendering|Material|SetVectorParameterValue _output_get "Color" (Math|Conversions|ToLinearColor(Color) _color) :!class /Script/Engine.MaterialInstanceDynamic)
  (Rendering|Material|SetMaterial (Variables|Default|GetTableComponent) 0 (Variables|Default|GetTableComponentDynamicMI)))

(fn ChangeSize
  (params (Coef :type Float%20%28single-precision%29))
  (Transformation|SetWorldScale3D (Variables|Default|GetGameCardShape) (* (Transformation|GetWorldScale (Variables|Default|GetGameCardShape)) Coef)))