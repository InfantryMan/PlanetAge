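; BP_GameView is an actor that sets up a board of planet-themed game cards on BeginPlay.
; It first builds a pool of planet structs with random materials and colors and a shared scale.
; It then spawns BP_GameCard actors in a three-wide grid computed from position settings.
; Each card independently draws a random name and planet struct, so repeats are possible.
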(event EventBeginPlay
  (CallFunction|GeneratePlanetStructArray)
  (Variables|Default|SetPositionSettings (Utilities|Struct|MakePositionSettings 250 -300 400 300))
  (CallFunction|SpawnGameCards))

(event Collision|EventActorBeginOverlap
  (params (OtherActor :type Actor%20Object%20Reference)))

(event EventTick
  (params (DeltaSeconds :type Float%20%28single-precision%29)))

(fn ConstructionScript)

(fn GeneratePlanetStruct
  (bind _materialarray (LocalVariables|GetMaterialArray))
  (bind _colorarray (LocalVariables|GetColorArray))
  (return (Utilities|Struct|MakePlanetStruct (Utilities|Array|Get(acopy) _materialarray (Utilities|Length->RandomNumber (Utilities|Array|Length _materialarray))) (Utilities|Array|Get(acopy) _colorarray (Utilities|Length->RandomNumber (Utilities|Array|Length _colorarray))) (LocalVariables|GetPlanetScale))))

(fn GeneratePlanetStructArray
  (for _index (range 0 (- (Variables|Default|GetPlanetStructNumber) 1))
    (bind _planetstructinstance (CallFunction|GeneratePlanetStruct))
    (Utilities|Array|AppendArray (Variables|Default|GetPlanetStructArray) (Utilities|Array|MakeArray _planetstructinstance))))

(fn SpawnGameCard
  (params (Transform :type Transform))
  (bind _planetnamearray (Variables|Default|GetPlanetNameArray))
  (bind _planetstructarray (Variables|Default|GetPlanetStructArray))
  (Game|SpawnActorfromClass "/Game/Blueprints/BP_GameCard.BP_GameCard_C" Transform "Undefined" 0 (Utilities|Array|Get(acopy) _planetnamearray (Utilities|Length->RandomNumber (Utilities|Array|Length _planetnamearray))) (Utilities|Array|Get(acopy) _planetstructarray (Utilities|Length->RandomNumber (Utilities|Array|Length _planetstructarray))) 0))

(fn SpawnGameCards
  (for _index (range 0 (- (Variables|Default|GetCardsNumber) 1))
    (CallFunction|SpawnGameCard (Math|Transform|MakeTransform (Math|Conversions|ToVector(Vector2D) (Utilities|Index->Position _index) 2e+01) "0,180.000000,0.000000"))))